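; BP_Torch is a pickup torch that the first-person player can collect when it is Pickable.
; An overlap box shows a prompt widget while the player is inside and hides it on exit.
; PickUp puts the torch mesh on the player's EquippedItem, reveals the linked GhostTorch and flags that the player has a torch, then destroys the actor.
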(event OnComponentEndOverlap(Box)
  (params (OverlappedComponent :type Primitive%20Component%20Object%20Reference) (OtherActor :type Actor%20Object%20Reference) (OtherComp :type Primitive%20Component%20Object%20Reference) (OtherBodyIndex :type Integer))
  ;[0.6427 1 0.549] Widget Visibility
  (Rendering|SetVisibility (Variables|Default|GetWidget) false false))

(event OnComponentBeginOverlap(Box)
  (params (OverlappedComponent :type Primitive%20Component%20Object%20Reference) (OtherActor :type Actor%20Object%20Reference) (OtherComp :type Primitive%20Component%20Object%20Reference) (OtherBodyIndex :type Integer) (bFromSweep :type Boolean) (SweepResult :type Hit%20Result%20Structure%20%28by%20ref%29))
  ;[0.6427 1 0.549] Widget Visibility
  (Utilities|Casting|CastToBP_FirstPersonCharacter OtherActor)
  (if (Variables|Default|GetPickable)
    (Rendering|SetVisibility (Variables|Default|GetWidget) true false)))

(event EventPickUp
  (bind _ghosttorch (Variables|Default|GetGhostTorch))
  (if (Variables|Default|GetPickable)
    (bind _asbp_first_person_character (Utilities|Casting|CastToBP_FirstPersonCharacter (Game|GetPlayerCharacter 0)))
    (Components|StaticMesh|SetStaticMesh (Variables|/Game/FirstPerson/Blueprints/BP_FirstPersonCharacter.BP_FirstPersonCharacter_C|GetEquippedItem _asbp_first_person_character) "/Game/Dungeon/Assets/Props/SM_Torch1.SM_Torch1")
    (Rendering|SetVisibility (Variables|/Game/BlueprintsImplemented/BP_GhostTorch.BP_GhostTorch_C|GetGhostTorch _ghosttorch) true false)
    (Variables|/Game/BlueprintsImplemented/BP_GhostTorch.BP_GhostTorch_C|SetPlayerHasTorch? _ghosttorch true)
    (Actor|DestroyActor)))

(fn ConstructionScript)