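; BP_Door is an interactable door that swings open and closed on its yaw axis.
; A trigger shows or hides a widget as overlaps begin and end.
; When CanOpen is true, each Interaction event alternates through a FlipFlop between playing the timeline from the start and reversing it.
; The timeline's float drives the door's relative rotation through a quarter turn, with its play rate derived from Duration.
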(event OnComponentBeginOverlap(Trigger)
  (params (OverlappedComponent :type Primitive%20Component%20Object%20Reference) (OtherActor :type Actor%20Object%20Reference) (OtherComp :type Primitive%20Component%20Object%20Reference) (OtherBodyIndex :type Integer) (bFromSweep :type Boolean) (SweepResult :type Hit%20Result%20Structure%20%28by%20ref%29))
  ;[0.6427 1 0.549] Widget Visibility
  (Rendering|SetVisibility (Variables|Widget|GetWidget) true false))

(event OnComponentEndOverlap(Trigger)
  (params (OverlappedComponent :type Primitive%20Component%20Object%20Reference) (OtherActor :type Actor%20Object%20Reference) (OtherComp :type Primitive%20Component%20Object%20Reference) (OtherBodyIndex :type Integer))
  ;[0.6427 1 0.549] Widget Visibility
  (Rendering|SetVisibility (Variables|Widget|GetWidget) false false))

(event EventBeginPlay
  (Components|Timeline|SetPlayRate (Variables|Default|GetTimeline) (/ 1.0 (Variables|Components|GetDuration))))

(event EventInteraction
  ;[1 1 1] OpeningDoor
  (if (Variables|Default|GetCanOpen)
    (Utilities|FlowControl|FlipFlop
      (:A
        (bind _dooranglefloat (Timeline|Timeline PlayFromStart)
          (:Update
            (Transformation|SetRelativeRotation (Variables|Default|GetDoor) (Math|Rotator|MakeRotator 0.0 0.0 (Math|Float|Lerp 0.0 -9e+01 _dooranglefloat)) false false))))
      (:B
        (Timeline|Timeline Reverse)))))

(fn ConstructionScript)