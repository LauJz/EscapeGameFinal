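; BP_Chest is a chest that opens once when the player interacts while holding a key, revealing a torch to pick up.
; A trigger overlap shows a widget to players without the key and hides it on exit.
; Interaction spawns a key mesh on the chest and rotates it by timeline, then plays opening animation and sounds.
; A timer then starts a second timeline that levitates the referenced torch and makes it pickable.
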(event OnComponentBeginOverlap(Trigger)
  (params (OverlappedComponent :type Primitive%20Component%20Object%20Reference) (OtherActor :type Actor%20Object%20Reference) (OtherComp :type Primitive%20Component%20Object%20Reference) (OtherBodyIndex :type Integer) (bFromSweep :type Boolean) (SweepResult :type Hit%20Result%20Structure%20%28by%20ref%29))
  ;[0.6427 1 0.549] Widget Visibility
  (bind _asbp_first_person_character (Utilities|Casting|CastToBP_FirstPersonCharacter OtherActor))
  (if (not (Variables|/Game/FirstPerson/Blueprints/BP_FirstPersonCharacter.BP_FirstPersonCharacter_C|GetHasKey _asbp_first_person_character))
    (Rendering|SetVisibility (Variables|Default|GetWidget) true false)))

(event OnComponentEndOverlap(Trigger)
  (params (OverlappedComponent :type Primitive%20Component%20Object%20Reference) (OtherActor :type Actor%20Object%20Reference) (OtherComp :type Primitive%20Component%20Object%20Reference) (OtherBodyIndex :type Integer))
  ;[0.6427 1 0.549] Widget Visibility
  (Rendering|SetVisibility (Variables|Default|GetWidget) false false))

(event Custom|OpeningChestEvent
  ;[1 0.4656 0.4656] Torche levitating
  (Audio|PlaySound2D "/Game/Audio/SFX_ChestOpening.SFX_ChestOpening" 1.0 1.0 0.0 0 0)
  (Components|Animation|PlayAnimation (Variables|Default|GetChest) "/Game/Dungeon/Assets/Chest/Chest_Anim_Armature_A_Open.Chest_Anim_Armature_A_Open" false)
  (Audio|PlaySound2D "/Game/Audio/SFX_AngelReveal.SFX_AngelReveal" 1.0 1.0 0.5 0 0)
  (Utilities|Time|SetTimerbyEvent (delegate Custom|RevealTorch) 2.0))

(event Custom|RevealTorch
  (bind _torche (Variables|Default|GetTorche))
  (bind _torch (Variables|/Game/BlueprintsImplemented/BP_Torch.BP_Torch_C|GetTorch _torche))
  (bind _returnvalue (Transformation|GetWorldLocation _torch))
  ;[1 0.4656 0.4656] Torche levitating
  (bind _newtrack_3 (Timeline|Torch%20Levitating Play)
    (:Update
      (Transformation|SetWorldLocation _torch (Math|Vector|MakeVector (.x _returnvalue) (.y _returnvalue) _newtrack_3) false false)
      (Variables|/Game/BlueprintsImplemented/BP_Torch.BP_Torch_C|SetPickable (Variables|Default|GetTorche) true))))

(event EventInteraction
  ;[1 0.6102 0.4073] Chest Opening
  (bind _asbp_first_person_character (Utilities|Casting|CastToBP_FirstPersonCharacter (Game|GetPlayerCharacter 0)))
  (if (Variables|/Game/FirstPerson/Blueprints/BP_FirstPersonCharacter.BP_FirstPersonCharacter_C|GetHasKey _asbp_first_person_character)
    (Utilities|FlowControl|DoOnce false
      (:Completed
        (bind _returnvalue (AddComponent|AddStaticMeshComponent false (Math|Transform|MakeTransform "55.000000,0.000000,40.000000" "0.000000,-180.000000,-90.000000" "1.000000,1.000000,1.000000")))
        (bind _output_get (Variables|Default|SetKey _returnvalue))
        (Transformation|AttachComponentToComponent _output_get (Variables|Default|GetChest) "None" "KeepWorld" "KeepWorld" "KeepRelative" true)
        (Collision|SetCollisionEnabled _output_get "NoCollision")
        (bind _keyopen (Timeline|KeyOpen Play)
          (:Update
            (Transformation|SetRelativeRotation (Variables|Default|GetKey) (Math|Rotator|MakeRotator (Math|Float|Lerp -9e+01 9e+01 _keyopen) (.pitch (Variables|/Script/Engine.SceneComponent|GetRelativeRotation (Variables|Default|GetKey))) (.yaw (Variables|/Script/Engine.SceneComponent|GetRelativeRotation (Variables|Default|GetKey)))) false false))
          (:Finished
            (Variables|Default|SetRotateKey true)
            (CallFunction|OpeningChestEvent)))))))

(fn ConstructionScript)